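; Projectile actor, fired by a player or tank, that damages whatever it hits and then destroys itself.
; The construction script copies the speed passed in by the shooter into the X component of the ProjectileMovement velocity and prints it for debugging.
; On hit, it applies fixed damage credited to the instigator's controller and prints the impact's wall-clock second and millisecond before destruction.
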(event `self.ReceiveBeginPlay`)

(event `self.ReceiveActorBeginOverlap`
  (params (OtherActor :type "Actor Object Reference")))

(event `self.ReceiveHit`
  (params (MyComp :type "PrimitiveComponent Object Reference") (Other :type "Actor Object Reference") (OtherComp :type "PrimitiveComponent Object Reference") (bSelfMoved :type Boolean) (HitLocation :type "Vector Structure") (HitNormal :type "Vector Structure") (NormalImpulse :type "Vector Structure") (Hit :type "HitResult Structure (by ref)"))
  (`GameplayStatics.ApplyDamage` Other 50.0 (`self.GetInstigatorController`) self)
  (`self.Print Time of Impact`) ; Sometimes useful for debugging
  (`self.K2_DestroyActor` self))

(fn `UserConstructionScript`
  (bind _initialspeedinput (`self.InitialSpeedInput`))
  ;[1 1 1] Set this bullet/projectile's Intial Speed to the speed input passed from the player/tank
  (`KismetSystemLibrary.PrintString` (`KismetStringLibrary.BuildString_Double` "Projectile Blueprint: " "" _initialspeedinput) true true (struct :`R` 0.264065 :`G` 1.0 :`B` 0.475065 :`A` 1.0) 5.0)
  (set `MovementComponent.Velocity` (`KismetMathLibrary.MakeVector` _initialspeedinput) (`self.ProjectileMovement`)))