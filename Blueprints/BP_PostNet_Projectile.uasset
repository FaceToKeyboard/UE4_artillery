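; Projectile actor that deals fixed damage to whatever it hits, then destroys itself.
; The construction script sets the movement component's X velocity from an initial speed input and prints that speed on screen.
; On hit, it applies damage credited to the instigator's controller and calls a macro that prints the impact's second and millisecond for debugging.
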(event `self.ReceiveBeginPlay`)

(event `self.ReceiveActorBeginOverlap`
  (params (OtherActor :type "Actor Object Reference")))

(event `self.ReceiveTick`
  (params (DeltaSeconds :type "Float (single-precision)")))

(event `self.ReceiveHit`
  (params (MyComp :type "PrimitiveComponent Object Reference") (Other :type "Actor Object Reference") (OtherComp :type "PrimitiveComponent Object Reference") (bSelfMoved :type Boolean) (HitLocation :type "Vector Structure") (HitNormal :type "Vector Structure") (NormalImpulse :type "Vector Structure") (Hit :type "HitResult Structure (by ref)"))
  (`GameplayStatics.ApplyDamage` Other 50.0 (`self.GetInstigatorController`) self)
  (`self.Print Time of Impact`
    (:`Output`
      (`self.K2_DestroyActor` self))))

(fn `UserConstructionScript`
  (bind _initialspeedinput (`self.InitialSpeedInput`))
  (`KismetSystemLibrary.PrintString` (`KismetStringLibrary.BuildString_Double` "Projectile Blueprint: " "" _initialspeedinput) true true (struct :`R` 0.264065 :`G` 1.0 :`B` 0.475065 :`A` 1.0) 5.0)
  (set `MovementComponent.Velocity` (`KismetMathLibrary.MakeVector` _initialspeedinput) (`self.MovementComp`)))